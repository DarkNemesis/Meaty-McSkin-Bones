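; Air vent fan actor that spins its Fan component while the linked Air reference reports an active vent state.
; BeginPlay caches the configured FanSpeed in OldSpeed.
; Tick yaws the fan by FanSpeed per frame, without delta-time scaling, then polls GetAirVentState to restore the cached speed or set it to zero.
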(event EventBeginPlay
  (Variables|Default|SetoldSpeed (Variables|Default|GetFanSpeed)))

(event EventTick
  (params (DeltaSeconds :type Float%20%28single-precision%29))
  (Transformation|AddRelativeRotation (Variables|Default|GetFan) (Math|Rotator|MakeRotator 0.0 0.0 (Variables|Default|GetFanSpeed)) false false)
  (bind _returnvalue (Class|EnvAirVent|GetAirVentState (Variables|Default|GetAir)))
  (if _returnvalue
    (Variables|Default|SetFanSpeed (Variables|Default|GetoldSpeed))
    (else
      (Variables|Default|SetFanSpeed 0.0))))

(fn ConstructionScript)